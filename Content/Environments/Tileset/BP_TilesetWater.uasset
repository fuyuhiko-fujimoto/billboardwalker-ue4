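; Water tile Blueprint for the tileset, a child of a parent class that supplies the parameter event.
; When a parameter is set, it runs the parent logic, then uses that value as an index into the Waters material array.
; The selected material is applied to the first slot of the Tile component, switching the water's look.
; BeginPlay, overlap and construction only pass through to the parent, and Tick is disabled.
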(event EventBeginPlay
  (|CallParentFunction))

(event Collision|EventActorBeginOverlap
  (params (OtherActor :type Actor%20Object%20Reference))
  (|CallParentFunction OtherActor))

(event EventTick
  (params (DeltaSeconds :type Float%20%28single-precision%29))
  (|CallParentFunction DeltaSeconds) ; This node is disabled and will not be called.\nDrag off pins to build functionality.
)

(event EventSetParameter
  (params (parameter :type Integer))
  (|CallParentFunction parameter)
  (CallFunction|SetTileMaterial))

(fn ConstructionScript
  (|CallParentFunction))

(fn SetTileMaterial
  (Rendering|Material|SetMaterial (Variables|Default|GetTile) 0 (Utilities|Array|Get(acopy) (Variables|WaterEdge|GetWaters) (Variables|Default|Getparameter_))))